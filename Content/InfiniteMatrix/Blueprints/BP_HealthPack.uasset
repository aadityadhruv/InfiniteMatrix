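; BP_HealthPack is a short-lived health pickup that heals the player by 10, capped at 100.
; An overlap on HealthIconCollision casts to BP_Player, sets the clamped Health, updates the HUD health bar and destroys the pack.
; The HUD value re-adds 10 to the updated Health before clamping, so the bar can read higher than actual Health.
; Tick destroys an uncollected pack five seconds after BeginPlay.
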(event `self.ReceiveBeginPlay`
  (set `self.startTime` (`self.GetGameTimeSinceCreation`)))

(event `self.ReceiveTick`
  (params (DeltaSeconds :type "Float (single-precision)"))
  (if (>= (- (`self.GetGameTimeSinceCreation`) (`self.startTime`)) 5.0)
    (`self.K2_DestroyActor`)))

(event `self.HealthIconCollision.OnComponentBeginOverlap`
  (params (OverlappedComponent :type "PrimitiveComponent Object Reference") (OtherActor :type "Actor Object Reference") (OtherComp :type "PrimitiveComponent Object Reference") (OtherBodyIndex :type Integer) (bFromSweep :type Boolean) (SweepResult :type "HitResult Structure (by ref)"))
  (bind _asbp_player (cast `/Game/InfiniteMatrix/Blueprints/BP_Player` OtherActor))
  (bind _returnvalue (`KismetMathLibrary.Clamp` (+ (`/Game/InfiniteMatrix/Blueprints/BP_Player.Health` _asbp_player) 10) 0 100))
  (set `/Game/InfiniteMatrix/Blueprints/BP_Player.Health` _returnvalue _asbp_player)
  (`/Game/InfiniteMatrix/UI/WBP_HUD.UpdateHealthBar` (`/Game/InfiniteMatrix/Blueprints/BP_Player.HUD` _asbp_player) (`KismetMathLibrary.Conv_IntToDouble` _returnvalue))
  (`self.K2_DestroyActor`))

(fn `UserConstructionScript`)