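; BP_Enemy is an enemy actor that damages the player on contact and removes itself after a short lifetime.
; It records its spawn time on BeginPlay and checks it each Tick to destroy itself once that time runs out.
; Overlapping BP_Player calls ProcessHit on the player and destroys the enemy.
; HandleCollision takes a projectile and destroys both it and the enemy.
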(event `self.ReceiveBeginPlay`
  (set `self.startTime` (`self.GetGameTimeSinceCreation`)))

(event `self.ReceiveTick`
  (params (DeltaSeconds :type "Float (single-precision)"))
  (if (>= (- (`self.GetGameTimeSinceCreation`) (`self.startTime`)) 5.0)
    (`self.K2_DestroyActor`)))

(event `self.ReceiveActorBeginOverlap`
  (params (OtherActor :type "Actor Object Reference"))
  (bind _asbp_player (cast `/Game/InfiniteMatrix/Blueprints/BP_Player` OtherActor))
  (`/Game/InfiniteMatrix/Blueprints/BP_Player.ProcessHit` _asbp_player)
  (`self.K2_DestroyActor`))

(event `/Game/InfiniteMatrix/Blueprints/CollidableObject.HandleCollision`
  (params (Projectile :type "/Game/InfiniteMatrix/Blueprints/BP_Projectile Object Reference"))
  (`self.K2_DestroyActor`)
  (`self.K2_DestroyActor` Projectile))

(fn `UserConstructionScript`)