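; BP_Projectile is a short-lived projectile actor that reports what it touches.
; It records its start time on BeginPlay, then checks elapsed time every Tick and destroys itself after five seconds.
; When its Sphere begins an overlap, it sends HandleCollisionMessage to the other actor with itself as the argument, leaving the response to that actor.
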(event `self.ReceiveBeginPlay`
  (set `self.startTime` (`self.GetGameTimeSinceCreation`)))

(event `self.ReceiveTick`
  (params (DeltaSeconds :type "Float (single-precision)"))
  (if (>= (- (`self.GetGameTimeSinceCreation`) (`self.startTime`)) 5.0)
    (`self.K2_DestroyActor`)))

(event `self.Sphere.OnComponentBeginOverlap`
  (params (OverlappedComponent :type "PrimitiveComponent Object Reference") (OtherActor :type "Actor Object Reference") (OtherComp :type "PrimitiveComponent Object Reference") (OtherBodyIndex :type Integer) (bFromSweep :type Boolean) (SweepResult :type "HitResult Structure (by ref)"))
  (message `/Game/InfiniteMatrix/Blueprints/CollidableObject.HandleCollision` OtherActor self))

(fn `UserConstructionScript`)